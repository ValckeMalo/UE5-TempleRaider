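; BP_Grabbable is an actor that can be looked at, grabbed and released.
; A SphereOutline component starts hidden, appears on Lookat and hides again on StopLookat.
; Grab and Release events call OnGrab and OnRelease, which turn physics simulation on the Object component on when grabbed and off when released.
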(event EventLookat
  (Development|SetHiddeninGame (Variables|Default|GetSphereOutline) false false))

(event EventStopLookat
  (Development|SetHiddeninGame (Variables|Default|GetSphereOutline) true false))

(event EventBeginPlay
  (Development|SetHiddeninGame (Variables|Default|GetSphereOutline) true false))

(event EventGrab
  (CallFunction|OnGrab))

(event EventRelease
  (CallFunction|OnRelease))

(fn ConstructionScript)

(fn OnGrab
  (Physics|SetSimulatePhysics (Variables|Default|GetObject) true))

(fn OnRelease
  (Physics|SetSimulatePhysics (Variables|Default|GetObject) false))